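; BP_BaseInteraction is a base actor for interactable objects with a world-space prompt widget showing its interaction text.
; Its trigger registers it with BP_Player on enter and exit and notifies the widget, which turns to face the camera every tick.
; Focus and Unfocus forward to the widget, and a visibility point supplies a location for visibility checks.
; Interact only prints a debug message naming the object and player.
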(event `self.ReceiveBeginPlay`
  (bind _asui_interaction_base (cast `/Game/UI/GameplayUI/UI_InteractionBase` (`WidgetComponent.GetWidget` (`self.Widget`))))
  (bind _output_get (set `self.WidgetInteraction` _asui_interaction_base))
  (bind _asui_interaction_text (cast `/Game/UI/GameplayUI/UI_InteractionText` _output_get))
  (`/Game/UI/GameplayUI/UI_InteractionText.SetInteractionText` _asui_interaction_text (`self.InteractionText`)))

(event `self.ReceiveTick`
  (params (DeltaSeconds :type "Float (single-precision)"))
  (`SceneComponent.K2_SetWorldRotation` (`self.Widget`) (`KismetMathLibrary.FindLookAtRotation` (`SceneComponent.K2_GetComponentLocation` (`self.Widget`)) (`PlayerCameraManager.GetCameraLocation` (`GameplayStatics.GetPlayerCameraManager` 0))) false false))

(event `self.Trigger.OnComponentBeginOverlap`
  (params (OverlappedComponent :type "PrimitiveComponent Object Reference") (OtherActor :type "Actor Object Reference") (OtherComp :type "PrimitiveComponent Object Reference") (OtherBodyIndex :type Integer) (bFromSweep :type Boolean) (SweepResult :type "HitResult Structure (by ref)"))
  (bind _asbp_player (cast `/Game/Blueprint/Character/BP_Player` OtherActor))
  (`/Game/Blueprint/Character/BP_Player.EnterInteractionRadius` _asbp_player self)
  (`/Game/UI/GameplayUI/UI_InteractionBase.OnInteractionRadiusEnter` (`self.WidgetInteraction`)))

(event `self.Trigger.OnComponentEndOverlap`
  (params (OverlappedComponent :type "PrimitiveComponent Object Reference") (OtherActor :type "Actor Object Reference") (OtherComp :type "PrimitiveComponent Object Reference") (OtherBodyIndex :type Integer))
  (bind _asbp_player (cast `/Game/Blueprint/Character/BP_Player` OtherActor))
  (`/Game/Blueprint/Character/BP_Player.ExitInteractionRadius` _asbp_player self)
  (`/Game/UI/GameplayUI/UI_InteractionBase.OnInteractionRadiusExit` (`self.WidgetInteraction`)))

(fn `Focus`
  (`/Game/UI/GameplayUI/UI_InteractionBase.OnFocus` (`self.WidgetInteraction`)))

(fn `GetVisibiltyCheckPoint`
  (returns (ReturnValue :type "Vector Structure"))
  (return (`SceneComponent.K2_GetComponentLocation` (`self.VisibilityPoint`))))

(fn `Interact`
  (params (Player :type "/Game/Blueprint/Character/BP_Player Object Reference"))
  (`KismetSystemLibrary.PrintString` (`KismetStringLibrary.Concat_StrStr` (`KismetSystemLibrary.GetDisplayName` self) " is interacted by " (`KismetSystemLibrary.GetDisplayName` Player))))

(fn `Unfocus`
  (`/Game/UI/GameplayUI/UI_InteractionBase.OnUnfocus` (`self.WidgetInteraction`)))

(fn `UserConstructionScript`)