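; Player controller that routes player input to the possessed BP_Player and tracks whether a gamepad is in use.
; On possession it caches the pawn as PlayerChara, then forwards move axes as world-axis movement and the Interact action to it.
; Any key press can update the gamepad flag and fire CallGamepadEvent, with a change check gated by AnyKeyAlreadyPressed.
; TogglePause is an empty stub.
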(event `Key|AnyKey` :consume false :paused true
  (params (Key :type "Key Structure"))
  (bind _returnvalue (`KismetInputLibrary.Key_IsGamepadKey` Key))
  (:`Pressed`
    (if (`self.AnyKeyAlreadyPressed`)
      (set `self.AnyKeyAlreadyPressed` true)
      (if (!= _returnvalue (`self.bIsUsingGamepad`))
        (bind _output_get (set `self.bIsUsingGamepad` _returnvalue :!label _label))
        (`self.GamepadEvent` _output_get))
      (else
        (goto _label)))))

(event `InputAxis|MoveRight` :consume false
  (params (AxisValue :type "Float (single-precision)"))
  (bind _playerchara (`self.PlayerChara`)
    (:`then`
      (`/Game/Blueprint/Character/BP_Player.AddInputMovement` _playerchara (0.0 1.0 0.0) AxisValue))
    (:`else`)))

(event `InputAxis|MoveUp` :consume false
  (params (AxisValue :type "Float (single-precision)"))
  (bind _playerchara (`self.PlayerChara`)
    (:`then`
      (`/Game/Blueprint/Character/BP_Player.AddInputMovement` _playerchara (1.0 0.0 0.0) AxisValue))
    (:`else`)))

(event `self.ReceivePossess`
  (params (PossessedPawn :type "Pawn Object Reference"))
  (bind _asbp_player (cast `/Game/Blueprint/Character/BP_Player` PossessedPawn))
  (set `self.PlayerChara` _asbp_player))

(event `InputAction|Interact`
  (params (Key :type "Key Structure"))
  (:`Pressed`
    (`/Game/Blueprint/Character/BP_Player.Interact` (`self.PlayerChara`))))

(fn `TogglePause`)

(fn `UserConstructionScript`)