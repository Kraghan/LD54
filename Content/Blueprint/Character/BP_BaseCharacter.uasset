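; BP_BaseCharacter is a base character that moves from accumulated input and turns to face the direction of that input.
; AddInputMovement sums normalized, scaled direction vectors into InputMovement.
; Each Tick, LookAtMoveDirection interpolates the control rotation toward that vector at RotationSpeed, then the vector is passed to CharacterMovement and cleared.
; Facing follows requested input, not velocity, and is left untouched when input is near zero.
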(event `self.ReceiveTick`
  (params (DeltaSeconds :type "Float (single-precision)"))
  (`self.LookAtMoveDirection` DeltaSeconds)
  (`PawnMovementComponent.AddInputVector` (`self.CharacterMovement`) (`self.InputMovement`) false)
  (set `self.InputMovement` (0.0 0.0 0.0)))

(fn `AddInputMovement`
  (params (MovementDirection :type "Vector Structure") (Scale :type "Float (double-precision)"))
  (set `self.InputMovement` (+ (* (`KismetMathLibrary.Normal` MovementDirection) Scale) (`self.InputMovement`))))

(fn `LookAtMoveDirection`
  (params (DeltaTime :type "Float (double-precision)"))
  (bind _returnvalue (`self.GetController`))
  (bind _returnvalue_2 (`self.K2_GetActorLocation`))
  (if (!= (`self.InputMovement`) (0.0 0.0 0.0))
    (`Controller.SetControlRotation` _returnvalue (`KismetMathLibrary.RInterpTo` (`Controller.GetControlRotation` _returnvalue) (`KismetMathLibrary.FindLookAtRotation` _returnvalue_2 (+ _returnvalue_2 (`self.InputMovement`))) DeltaTime (`self.RotationSpeed`)))))

(fn `UserConstructionScript`)