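; Player camera manager that follows BP_Player at a fixed height, rotation and FOV, using a screen-space dead zone.
; BlueprintUpdateCamera projects the mesh's CameraTarget socket to screen ratios, and IsOutOfBounds tests them against HardDeadZoneSize.
; When outside, GetDistance offsets the 2D target by the difference between Camera-channel trace hits toward the socket and along camera forward.
; The 2D location eases toward that target with VInterpTo at SmoothSpeed.
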(event `self.ReceiveBeginPlay`
  (bind (_returnvalue_x _returnvalue_y) (`KismetMathLibrary.BreakVector` (`self.K2_GetActorLocation` (`GameplayStatics.GetPlayerPawn` 0))))
  (set `self.CurrentCameraLocation2D` (+ (`KismetMathLibrary.MakeVector2D` _returnvalue_x _returnvalue_y) (`self.CurrentCameraLocation2D`))))

(event `self.ReceiveTick`
  (params (DeltaSeconds :type "Float (single-precision)")))

(fn `BlueprintUpdateCamera`
  (params (CameraTarget :type "Actor Object Reference"))
  (returns (NewCameraLocation :type "Vector Structure") (NewCameraRotation :type "Rotator Structure") (NewCameraFOV :type "Float (single-precision)") (ReturnValue :type Boolean))
  (locals (PlayerScreenPosInRatio :type "Vector2D Structure") (NewLocation2D :type "Vector2D Structure") (PlayerScreenPos :type "Vector2D Structure") (bIsOutBounds :type Boolean))
  (bind (_currentcameralocation2d_x _currentcameralocation2d_y) (`KismetMathLibrary.BreakVector2D` (`self.CurrentCameraLocation2D`)))
  (bind (_currentcameralocation2d_x_2 _currentcameralocation2d_y_2) (`KismetMathLibrary.BreakVector2D` (`self.CurrentCameraLocation2D`)))
  (bind (_newcameratarget_x _newcameratarget_y) (`KismetMathLibrary.BreakVector2D` (`self.NewCameraTarget`)))
  (bind (_returnvalue_x _returnvalue_y) (`KismetMathLibrary.BreakVector` (`KismetMathLibrary.VInterpTo` (`KismetMathLibrary.MakeVector` _currentcameralocation2d_x_2 _currentcameralocation2d_y_2) (`KismetMathLibrary.MakeVector` _newcameratarget_x _newcameratarget_y) (- (`GameplayStatics.GetTimeSeconds`) (`self.LastTime`)) (`self.SmoothSpeed`))))
  (bind _asbp_player (cast `/Game/Blueprint/Character/BP_Player` (`GameplayStatics.GetPlayerPawn` 0)))
  (bind _returnvalue (`SceneComponent.GetSocketLocation` (`Character.Mesh` _asbp_player) "CameraTarget"))
  (bind (_screenposition _returnvalue_2) (`GameplayStatics.ProjectWorldToScreen` (`self.GetOwningPlayerController`) _returnvalue))
  (bind _output_get (set `local.PlayerScreenPos` _screenposition))
  (set `local.PlayerScreenPosInRatio` (/ _output_get (`WidgetLayoutLibrary.GetViewportSize`)))
  (if _returnvalue_2
    (if (`self.IsOutOfBounds` (`self.HardDeadZoneSize`) (`local.PlayerScreenPosInRatio`))
      (set `self.NewCameraTarget` (+ (`self.GetDistance` _returnvalue) (`self.CurrentCameraLocation2D`))))
    (set `self.CurrentCameraLocation2D` (`KismetMathLibrary.MakeVector2D` _returnvalue_x _returnvalue_y))
    (else
      (set `self.NewCameraTarget` (`self.CurrentCameraLocation2D`))))
  (set `self.LastTime` (`GameplayStatics.GetTimeSeconds`))
  (return (`KismetMathLibrary.MakeVector` _currentcameralocation2d_x _currentcameralocation2d_y (`self.CameraHeigth`)) (`self.CameraRotation`) (`self.FOV`) true))

(fn `GetDistance`
  (params (End :type "Vector Structure"))
  (returns (NewParam :type "Vector2D Structure"))
  (locals (Start :type "Vector Structure"))
  (bind (_currentcameralocation2d_x _currentcameralocation2d_y) (`KismetMathLibrary.BreakVector2D` (`self.CurrentCameraLocation2D`)))
  (bind _start (`local.Start`))
  (bind _output_get (set `local.Start` (`KismetMathLibrary.MakeVector` _currentcameralocation2d_x _currentcameralocation2d_y (`self.CameraHeigth`))))
  (bind _outhit (`KismetSystemLibrary.LineTraceSingle` _output_get End "TraceTypeQuery2"))
  (bind _outhit_2 (`KismetSystemLibrary.LineTraceSingle` _start (+ _start (* (`KismetMathLibrary.GetForwardVector` (`self.CameraRotation`)) 100000000.0)) "TraceTypeQuery2"))
  (bind (_returnvalue_x _returnvalue_y) (`KismetMathLibrary.BreakVector` (- (`.Location` (`GameplayStatics.BreakHitResult` _outhit)) (`.Location` (`GameplayStatics.BreakHitResult` _outhit_2)))))
  (return (`KismetMathLibrary.MakeVector2D` _returnvalue_x _returnvalue_y)))

(fn `IsOutOfBounds`
  (params (DeadZone :type "Vector2D Structure") (ScreenPos :type "Vector2D Structure"))
  (returns (bIsOutOfBound :type Boolean) (FinalPos :type "Vector2D Structure"))
  (locals (ResultPos :type "Vector2D Structure") (bIsOutBounds :type Boolean))
  (bind (_deadzone_x _deadzone_y) (`KismetMathLibrary.BreakVector2D` (`local.DeadZone`)))
  (bind _deadzone_x_2 (`KismetMathLibrary.BreakVector2D` (`local.DeadZone`)))
  (bind (_deadzone_x_3 _deadzone_y_2) (`KismetMathLibrary.BreakVector2D` (`local.DeadZone`)))
  (bind (_deadzone_x_4 _deadzone_y_3) (`KismetMathLibrary.BreakVector2D` (`local.DeadZone`)))
  (bind _deadzone_x_5 (`KismetMathLibrary.BreakVector2D` (`local.DeadZone`)))
  (bind _screenpos_x (`KismetMathLibrary.BreakVector2D` (`local.ScreenPos`)))
  (bind _screenpos_x_2 (`KismetMathLibrary.BreakVector2D` (`local.ScreenPos`)))
  (bind _resultpos_x (`KismetMathLibrary.BreakVector2D` (`local.ResultPos`)))
  (bind (_screenpos_x_3 _screenpos_y) (`KismetMathLibrary.BreakVector2D` (`local.ScreenPos`)))
  (bind _deadzone_x_6 (`KismetMathLibrary.BreakVector2D` (`local.DeadZone`)))
  (bind (_screenpos_x_4 _screenpos_y_2) (`KismetMathLibrary.BreakVector2D` (`local.ScreenPos`)))
  (bind _resultpos_x_2 (`KismetMathLibrary.BreakVector2D` (`local.ResultPos`)))
  (bind (_resultpos_x_3 _resultpos_y) (`KismetMathLibrary.BreakVector2D` (`local.ResultPos`)))
  (bind (_resultpos_x_4 _resultpos_y_2) (`KismetMathLibrary.BreakVector2D` (`local.ResultPos`)))
  (bind _deadzone_x_7 (`KismetMathLibrary.BreakVector2D` (`local.DeadZone`)))
  (bind (_deadzone_x_8 _deadzone_y_4) (`KismetMathLibrary.BreakVector2D` (`local.DeadZone`)))
  (set `local.ResultPos` ScreenPos)
  ;[1 1 1] < deadzone X
  (if (< _screenpos_x _deadzone_x_2)
    (set `local.ResultPos` (`KismetMathLibrary.MakeVector2D` _deadzone_x_5 _resultpos_y_2))
    (set `local.bIsOutBounds` true))
  ;[1 1 1] > deadzone X
  (if (> _screenpos_x_2 (- 1.0 _deadzone_x_6))
    (set `local.ResultPos` (`KismetMathLibrary.MakeVector2D` (- 1.0 _deadzone_x_7) _resultpos_y))
    (set `local.bIsOutBounds` true))
  ;[1 1 1] < deadzone Y
  (if (< _screenpos_y _deadzone_y_4)
    (set `local.ResultPos` (`KismetMathLibrary.MakeVector2D` _resultpos_x _deadzone_y_2))
    (set `local.bIsOutBounds` true))
  ;[1 1 1] > deadzone Y
  (if (> _screenpos_y_2 (- 1.0 _deadzone_y_3))
    (set `local.ResultPos` (`KismetMathLibrary.MakeVector2D` _resultpos_x_2 (- 1.0 _deadzone_y)))
    (set `local.bIsOutBounds` true))
  (return (`local.bIsOutBounds`) (`local.ResultPos`)))

(fn `UserConstructionScript`)